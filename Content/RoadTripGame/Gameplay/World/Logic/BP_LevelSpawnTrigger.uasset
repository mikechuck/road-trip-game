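; BP_LevelSpawnTrigger is a world trigger actor that requests the next level chunk from BP_GameplayGameMode when overlapped.
; Both actor and Trigger component overlaps call TriggerNextChunkLoad on the server, with no filter on the overlapping actor.
; On BeginPlay, a server RPC copies the game mode's ChunkCount into an unset TriggerValue via multicast.
; TriggerValue is only printed for debugging, not checked on overlap.
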(event `self.ReceiveBeginPlay`
  (`self.SRPC_GetTiggerValue`))

(event `self.Trigger.OnComponentBeginOverlap`
  (params (OverlappedComponent :type "PrimitiveComponent Object Reference") (OtherActor :type "Actor Object Reference") (OtherComp :type "PrimitiveComponent Object Reference") (OtherBodyIndex :type Integer) (bFromSweep :type Boolean) (SweepResult :type "HitResult Structure (by ref)"))
  (`KismetSystemLibrary.PrintString` "Hello" true true (struct :`G` 0.66 :`B` 1.0 :`A` 1.0) 200.0 :!label _label)
  (if (`KismetSystemLibrary.IsServer`)
    (bind _asbp_gameplay_game_mode (cast `/Game/RoadTripGame/Gameplay/BP_GameplayGameMode` (`GameplayStatics.GetGameMode`)))
    (`/Game/RoadTripGame/Gameplay/BP_GameplayGameMode.TriggerNextChunkLoad` _asbp_gameplay_game_mode)))

(event `self.ReceiveActorBeginOverlap`
  (params (OtherActor :type "Actor Object Reference"))
  (goto _label))

(event `SRPC_GetTiggerValue`
  (if (== (`self.TriggerValue`) 0)
    (bind _asbp_gameplay_game_mode (cast `/Game/RoadTripGame/Gameplay/BP_GameplayGameMode` (`GameplayStatics.GetGameMode`)))
    (`self.Multicast_SetTriggerValue` (`/Game/RoadTripGame/Gameplay/BP_GameplayGameMode.ChunkCount` _asbp_gameplay_game_mode))))

(event `Multicast_SetTriggerValue`
  (params (NewTriggerValue :type Integer))
  (set `self.TriggerValue` NewTriggerValue)
  (`KismetSystemLibrary.PrintString` (`KismetStringLibrary.Concat_StrStr` "Set the trigger value to" (`KismetStringLibrary.Conv_IntToString` (`self.TriggerValue`))) true true (struct :`G` 0.66 :`B` 1.0 :`A` 1.0) 200.0))

(fn `UserConstructionScript`)