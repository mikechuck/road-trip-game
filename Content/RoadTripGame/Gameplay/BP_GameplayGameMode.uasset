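; BP_GameplayGameMode is the road trip game's gameplay game mode, coordinating level-chunk streaming across connected players.
; PostLogin records each new controller and calls CRPCSpawnFirstStreamLevel on its BP_GameplayPlayerController to start that player's first level.
; TriggerNextChunkLoad increments ChunkCount, then passes it to every player controller through MulticastSpawnNewStreamLevel.
; That broadcast iterates controllers by index rather than using the stored ConnectedPlayers list.
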(event `self.ReceiveBeginPlay`)

(event `self.K2_PostLogin`
  (params (NewPlayer :type "PlayerController Object Reference"))
  (`KismetArrayLibrary.Array_Add` (`self.ConnectedPlayers`) NewPlayer)
  (bind _asbp_gameplay_player_controller (cast `/Game/RoadTripGame/Gameplay/Player/BP_GameplayPlayerController` NewPlayer))
  (`/Game/RoadTripGame/Gameplay/Player/BP_GameplayPlayerController.CRPC_SpawnFirstStreamLevel` _asbp_gameplay_player_controller))

(fn `TriggerNextChunkLoad`
  (`KismetSystemLibrary.PrintString` "increementing chunk count")
  (bind _result (`/Engine/EditorBlueprintResources/StandardMacros.IncrementInt` (`self.ChunkCount`))
    (:`  `
      (set `self.ChunkCount` _result)
      (for _index (range (`GameplayStatics.GetNumPlayerControllers`))
        (bind _asbp_gameplay_player_controller (cast `/Game/RoadTripGame/Gameplay/Player/BP_GameplayPlayerController` (`GameplayStatics.GetPlayerController` _index)))
        (`/Game/RoadTripGame/Gameplay/Player/BP_GameplayPlayerController.Multicast_SpawnNewStreamLevel` _asbp_gameplay_player_controller (`self.ChunkCount`))))))

(fn `UserConstructionScript`)