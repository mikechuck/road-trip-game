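; BP_PlayerCharacter is the player's character, providing movement and look controls through Enhanced Input.
; On BeginPlay it casts the first player controller to BP_GameplayPlayerController and adds the IMC_Player mapping context.
; IA_Move drives movement input along forward and right vectors derived from control rotation, with pitch zeroed so movement stays level.
; IA_Look feeds controller yaw and pitch.
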(event `self.ReceiveBeginPlay`
  (bind _asbp_gameplay_player_controller (cast `/Game/RoadTripGame/Gameplay/Player/BP_GameplayPlayerController` (`GameplayStatics.GetPlayerController` 0)))
  (bind _returnvalue (pcsubsystem `EnhancedInputLocalPlayerSubsystem` _asbp_gameplay_player_controller))
  (`/Engine/EditorBlueprintResources/StandardMacros.IsValid` _returnvalue
    (:`Is Valid`
      (`EnhancedInputSubsystemInterface.AddMappingContext` _returnvalue "/Game/RoadTripGame/Gameplay/Player/Inputs/IMC_Player.IMC_Player" 0 (struct)))))

(event `EnhancedInput|/Game/RoadTripGame/Gameplay/Player/Inputs/IA_Move`
  (params (ActionValue :type "Vector2D Structure") (ElapsedSeconds :type "Float (double-precision)") (TriggeredSeconds :type "Float (double-precision)") (InputAction :type "InputAction Object Reference" :default "/Game/RoadTripGame/Gameplay/Player/Inputs/IA_Move.IA_Move"))
  (bind (_returnvalue_roll _returnvalue_pitch _returnvalue_yaw) (`KismetMathLibrary.BreakRotator` (`self.GetControlRotation`)))
  (bind (_returnvalue_roll_2 _returnvalue_pitch_2 _returnvalue_yaw_2) (`KismetMathLibrary.BreakRotator` (`self.GetControlRotation`)))
  ;[0.1094 0.1094 0.1094] Input Actions
  (:`Triggered`
    (`self.AddMovementInput` (`KismetMathLibrary.GetRightVector` (`KismetMathLibrary.MakeRotator` _returnvalue_roll 0.0 _returnvalue_yaw)) ActionValue_X)
    (`self.AddMovementInput` (`KismetMathLibrary.GetForwardVector` (`KismetMathLibrary.MakeRotator` 0.0 0.0 _returnvalue_yaw_2)) ActionValue_Y)))

(event `EnhancedInput|/Game/RoadTripGame/Gameplay/Player/Inputs/IA_Look`
  (params (ActionValue :type "Vector2D Structure") (ElapsedSeconds :type "Float (double-precision)") (TriggeredSeconds :type "Float (double-precision)") (InputAction :type "InputAction Object Reference" :default "/Game/RoadTripGame/Gameplay/Player/Inputs/IA_Look.IA_Look"))
  ;[0.1094 0.1094 0.1094] Input Actions
  (:`Triggered`
    (`self.AddControllerYawInput` ActionValue_X)
    (bind _result (`/Engine/EditorBlueprintResources/StandardMacros.NegateFloat` ActionValue_Y)
      (:`  `
        (`self.AddControllerPitchInput` _result)))))

(fn `UserConstructionScript`)